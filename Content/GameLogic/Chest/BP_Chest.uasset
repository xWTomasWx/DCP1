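; BP_Chest is a one-time interactable loot chest that randomly rewards the player with either a key or coins.
; Interact swaps the mesh to the empty chest, marks it opened, then rolls 50/50 between adding a key to the third-person character's KeysInventory and adding CoinsToGive to its Coins.
; The reward goes to player 0's character, with a debug print of the result, and CanInteract returns false once opened.
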(event `/Game/GameLogic/Chest/BPI_Interactable.Interact`
  (params (Caller :type "Actor Object Reference"))
  (if (not (`self.bOpened`))
    (`StaticMeshComponent.SetStaticMesh` (`self.Chest`) "/Game/Stylised_Dungeon_Pack/Meshes/Furniture/SM_Chest_Empty.SM_Chest_Empty")
    (set `self.bOpened` true)
    (if (== (`KismetMathLibrary.RandomIntegerInRange` 0 1) 0)
      (bind _asbp_third_person_character (cast `/Game/ThirdPerson/Blueprints/BP_ThirdPersonCharacter` (`GameplayStatics.GetPlayerCharacter` 0)))
      (`KismetArrayLibrary.Array_Add` (`/Game/ThirdPerson/Blueprints/BP_ThirdPersonCharacter.KeysInventory` _asbp_third_person_character) "NewEnumerator0")
      (`KismetSystemLibrary.PrintString` "Consiguio la llave")
      (else
        (bind _asbp_third_person_character_2 (cast `/Game/ThirdPerson/Blueprints/BP_ThirdPersonCharacter` (`GameplayStatics.GetPlayerCharacter` 0)))
        (bind _output_get (set `/Game/ThirdPerson/Blueprints/BP_ThirdPersonCharacter.Coins` (+ (`self.CoinsToGive`) (`/Game/ThirdPerson/Blueprints/BP_ThirdPersonCharacter.Coins` _asbp_third_person_character_2)) _asbp_third_person_character_2))
        (`KismetSystemLibrary.PrintString` (`KismetStringLibrary.Conv_IntToString` _output_get))))))

(fn `CanInteract`
  (params (Caller :type "Actor Object Reference"))
  (returns (ReturnValue :type Boolean))
  (return (not (`self.bOpened`))))

(fn `UserConstructionScript`)