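; BP_Door is an interactive door that the player can swing or destroy.
; A box trigger enables input and shows the Interfaz prompt while BP_ThirdPersonCharacter overlaps it.
; F, gated by BoolOpen, plays a timeline yaw lerp, then a second timeline reverses it after a delay and re-arms the flag.
; E destroys the door, and an unfinished key-inventory check is left unconnected.
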(event `self.Box.OnComponentBeginOverlap`
  (params (OverlappedComponent :type "PrimitiveComponent Object Reference") (OtherActor :type "Actor Object Reference") (OtherComp :type "PrimitiveComponent Object Reference") (OtherBodyIndex :type Integer) (bFromSweep :type Boolean) (SweepResult :type "HitResult Structure (by ref)"))
  ; cuadradito para mostrar texto de apertura (Se puede reutilizar en otros bluprints ono)
  (cast `/Game/ThirdPerson/Blueprints/BP_ThirdPersonCharacter` OtherActor)
  (`self.EnableInput` (`GameplayStatics.GetPlayerController` 0))
  (bind _returnvalue (`|CreateWidget` "/Game/GameLogic/Tools/NormalDoor/Interfaz.Interfaz_C"))
  (`UserWidget.AddToViewport` _returnvalue 0))

(event `Key|E`
  (params (Key :type "Key Structure"))
  ; Boton de Destruccion de puerta >< (poner la tecla de ataque)
  (:`Pressed`
    (`self.K2_DestroyActor`)))

(event `self.Box.OnComponentEndOverlap`
  (params (OverlappedComponent :type "PrimitiveComponent Object Reference") (OtherActor :type "Actor Object Reference") (OtherComp :type "PrimitiveComponent Object Reference") (OtherBodyIndex :type Integer))
  ; cuadradito para mostrar texto de apertura (Se puede reutilizar en otros bluprints ono)
  (cast `/Game/ThirdPerson/Blueprints/BP_ThirdPersonCharacter` OtherActor)
  (`self.DisableInput` null)
  (`Widget.RemoveFromParent` (stale `self.Box.OnComponentBeginOverlap` _returnvalue)))

(event `Key|F`
  (params (Key :type "Key Structure"))
  ; Boton Apertura Puerta. (Cosnultar animacion de cierre hasta el momento abre sin problema yeppie)
  (:`Pressed`
    (if (`self.BoolOpen`)
      (set `self.BoolOpen` false)
      (bind (_direction _animacion_apertura) (`Timeline|Timeline` :!via `PlayFromStart`)
        (:`Update`
          (`SceneComponent.K2_SetRelativeRotation` (`self.Door`) (`KismetMathLibrary.MakeRotator` 0.0 0.0 (`KismetMathLibrary.Lerp` (`self.DoorOpen`) (`self.DoorClose`) _animacion_apertura)) false false)
          (`KismetSystemLibrary.Delay` 3.0)
          (bind (_direction_2 _animacion_apertura_2) (`Timeline|Cronograma` :!via `PlayFromStart`)
            (:`Update`
              (`SceneComponent.K2_SetRelativeRotation` (`self.Door`) (`KismetMathLibrary.MakeRotator` 0.0 0.0 (`KismetMathLibrary.Lerp` (`self.DoorClose`) (`self.DoorOpen`) _animacion_apertura_2)) false false)
              (set `self.BoolOpen` true))))))))

(fn `UserConstructionScript`)