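; Enemy character that chases the player once spotted and punches in melee, and is destroyed when damage depletes its health.
; PawnSensing sets IsSeeing, which is never cleared, and triggers Follow to AI-move toward player 0; until then, Tick halts movement.
; On arrival it plays a punch montage and immediately damages whatever a debug-drawn line trace between StartAttack and EndAttack hits.
; CanAttack blocks further attacks for the montage's duration.
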(event `self.ReceiveTick`
  (params (DeltaSeconds :type "Float (single-precision)"))
  (if (not (`self.isSeeing`))
    (`MovementComponent.StopMovementImmediately` (`self.CharacterMovement`))))

(event `self.ReceiveAnyDamage`
  (params (Damage :type "Float (single-precision)") (DamageType :type "DamageType Object Reference") (InstigatedBy :type "Controller Object Reference") (DamageCauser :type "Actor Object Reference"))
  (bind _returnvalue (> (`self.Health`) 0.0))
  (if _returnvalue
    (set `self.Health` (- (`self.Health`) Damage))
    (if (not _returnvalue)
      (`self.K2_DestroyActor`))))

(event `self.PawnSensing.OnSeePawn`
  (params (Pawn :type "Pawn Object Reference"))
  (set `self.isSeeing` true)
  (`self.Follow`))

(event `Follow`
  (if (`self.isSeeing`)
    (`|AIMoveTo` self (0.0 0.0 0.0) (`GameplayStatics.GetPlayerCharacter` 0) 100.0
      (:`OnSuccess`
        (if (`self.canAttack`)
          (set `self.canAttack` false)
          (bind _returnvalue (`self.PlayAnimMontage` "/Game/Characters/Enemy/Animations/Paired_CounterPunch_PalmStrike_Att1_Montage.Paired_CounterPunch_PalmStrike_Att1_Montage"))
          (bind _outhit (`KismetSystemLibrary.LineTraceSingle` :`Start` (`SceneComponent.GetSocketLocation` (`self.StartAttack`) "None") :`End` (`SceneComponent.GetSocketLocation` (`self.EndAttack`) "None") :`TraceChannel` "TraceTypeQuery1" :`DrawDebugType` "ForDuration"))
          (`GameplayStatics.ApplyDamage` (`.HitActor` (`GameplayStatics.BreakHitResult` _outhit)) 30.0)
          (`KismetSystemLibrary.Delay` _returnvalue)
          (set `self.canAttack` true))))))

(fn `UserConstructionScript`)